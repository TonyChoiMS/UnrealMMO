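; Player character Blueprint that handles taking damage and dying.
; AnyDamage subtracts the damage from PlayerHP and, while HP remains, plays a hit montage with sound and particle feedback.
; At zero or below it plays the Martin_Die animation directly on the mesh, disables movement and spawns death sound and effect.
; Both branches print debug strings, and no guard stops the death sequence repeating on further damage.
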(event EventBeginPlay)

(event Collision|EventActorBeginOverlap
  (params (OtherActor :type Actor%20Object%20Reference)))

(event EventTick
  (params (DeltaSeconds :type Float%20%28single-precision%29)))

(event Game|Damage|EventAnyDamage
  (params (Damage :type Float%20%28single-precision%29) (DamageType :type Damage%20Type%20Object%20Reference) (InstigatedBy :type Controller%20Object%20Reference) (DamageCauser :type Actor%20Object%20Reference))
  (bind _capsulecomponent (Variables|Default|GetCapsuleComponent))
  (bind _capsulecomponent_2 (Variables|Default|GetCapsuleComponent))
  (bind _returnvalue (Transformation|GetWorldLocation _capsulecomponent_2))
  (bind _returnvalue_2 (Transformation|GetWorldLocation _capsulecomponent))
  (bind _output_get (Variables|Default|SetPlayerHP (- (Variables|Default|GetPlayerHP) Damage)))
  (if (> _output_get 0.0)
    (Development|PrintString (Utilities|String|ToString(Float) _output_get))
    (Animation|PlayAnimMontage "/Game/TimeTravel/Animations/PlayerTakeHitMontage.PlayerTakeHitMontage" 1.0 "None")
    (Audio|SpawnSoundatLocation "/Game/TimeTravel/Sounds/PlayerTakeHitSoundCue.PlayerTakeHitSoundCue" _returnvalue_2 "0, 0, 0" 1.0 1.0 0.0 0 0)
    (Effects|SpawnEmitteratLocation "/Game/FXVarietyPack/Particles/P_ky_hit1.P_ky_hit1" _returnvalue)
    (else
      (Development|PrintString "Player Dead")
      (Components|Animation|PlayAnimation (Variables|Character|GetMesh) "/Game/TimeTravel/Animations/Martin_Die.Martin_Die" false)
      (Pawn|Components|CharacterMovement|DisableMovement (Variables|Character|GetCharacterMovement))
      (Audio|SpawnSoundatLocation "/Game/TimeTravel/Sounds/PlayerDeathSoundCue.PlayerDeathSoundCue" _returnvalue_2 "0, 0, 0" 1.0 1.0 0.0 0 0)
      (Effects|SpawnEmitteratLocation "/Game/InfinityBladeGrassLands/Effects/FX_Mobile/ICE/combat/P_Buff_ShoutFreeze_02.P_Buff_ShoutFreeze_02" _returnvalue))))

(fn ConstructionScript)