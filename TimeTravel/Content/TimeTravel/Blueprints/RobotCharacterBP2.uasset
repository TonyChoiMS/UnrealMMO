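; RobotCharacterBP2 is a robot character Blueprint that gives its mesh a light red enemy look.
; The construction script calls the parent's, then creates dynamic instances of the enemy body and face materials on the first two mesh slots and tints both the same color.
; The event graph holds only disabled default events, so the Blueprint adds no runtime logic of its own.
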(event EventBeginPlay
  (|CallParentFunction) ; 지금 이 노드는 비활성 상태입니다. \n핀을 끌어서 다른 노드를 연결하면 활성화됩니다.
)

(event Collision|EventActorBeginOverlap
  (params (OtherActor :type Actor%20Object%20Reference))
  (|CallParentFunction OtherActor) ; 지금 이 노드는 비활성 상태입니다. \n핀을 끌어서 다른 노드를 연결하면 활성화됩니다.
)

(event EventTick
  (params (DeltaSeconds :type Float%20%28single-precision%29))
  (|CallParentFunction DeltaSeconds) ; 지금 이 노드는 비활성 상태입니다. \n핀을 끌어서 다른 노드를 연결하면 활성화됩니다.
)

(fn ConstructionScript
  (|CallParentFunction)
  (bind _returnvalue (Rendering|Material|CreateDynamicMaterialInstance (Variables|Character|GetMesh) 0 "/Game/TimeTravel/Robot/Enemy_Body_Mat.Enemy_Body_Mat" "None" :!class /Script/Engine.PrimitiveComponent))
  (Rendering|Material|SetVectorParameterValue _returnvalue "BodyColor" (Utilities|Struct|MakeLinearColor 1.0 0.5 0.5 1.0) :!class /Script/Engine.MaterialInstanceDynamic)
  (bind _returnvalue_2 (Rendering|Material|CreateDynamicMaterialInstance (Variables|Character|GetMesh) 1 "/Game/TimeTravel/Robot/Enemy_Face_Mat.Enemy_Face_Mat" "None" :!class /Script/Engine.PrimitiveComponent))
  (Rendering|Material|SetVectorParameterValue _returnvalue_2 "FaceColor" (Utilities|Struct|MakeLinearColor 1.0 0.5 0.5 1.0) :!class /Script/Engine.MaterialInstanceDynamic))